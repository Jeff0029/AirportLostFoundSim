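; Lost item actor that picks a random identity from the LostItems data table, weighted by DropChance, when spawned as new.
; The chosen row sets its mesh and enables physics, and faster hits play a floor-drop sound.
; HideFromView disables physics, visibility and collision, while DropAtLocation spawns a non-new replacement carrying item and owner data, then destroys itself.
; SnapToSocket is empty, with its attach logic left disconnected.
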(event OnComponentHit(lostObject)
  (params (HitComponent :type Primitive%20Component%20Object%20Reference) (OtherActor :type Actor%20Object%20Reference) (OtherComp :type Primitive%20Component%20Object%20Reference) (NormalImpulse :type Vector :default "0, 0, 0") (Hit :type Hit%20Result%20Structure%20%28by%20ref%29))
  (if (> (Math|Vector|VectorLength (Transformation|GetComponentVelocity HitComponent)) 5e+01)
    (Audio|PlaySoundatLocation "/Game/Audio/objectDropOnFloor.objectDropOnFloor" (Transformation|GetActorLocation) "0, 0, 0" 0.4 1.0 0.0 "/Game/Audio/ItemHitFloor.ItemHitFloor" 0 0)))

(event EventBeginPlay
  (if (Variables|Default|GetIsNew)
    (CallFunction|SetupLostItem)))

(event Collision|EventActorBeginOverlap
  (params (OtherActor :type Actor%20Object%20Reference)))

(event EventTick
  (params (DeltaSeconds :type Float%20%28single-precision%29)))

(fn ConstructionScript)

(fn SetupLostItem
  (bind _outrownames (DataTable|GetDataTableRowNames "/Game/Data/lostItems.lostItems"))
  (for _array_element _outrownames ; Add up all the chance
    (bind _returnvalue (Utilities|GetDataTableRow "/Game/Data/lostItems.lostItems" _array_element)
      (:then
        (LocalVariables|SettotalChance (+ (Utilities|Struct|BreakItems _returnvalue) (LocalVariables|GettotalChance))))))
  (LocalVariables|SetgeneratedChance (Math|Random|RandomFloatinRange 0.0 (LocalVariables|GettotalChance)))
  (for _array_element_2 _outrownames
    (bind _returnvalue_2 (Utilities|GetDataTableRow "/Game/Data/lostItems.lostItems" _array_element_2)
      (:then
        (LocalVariables|SetcurChanceGroup (+ (Utilities|Struct|BreakItems _returnvalue_2) (LocalVariables|GetcurChanceGroup)))
        (if (<= (LocalVariables|GetgeneratedChance) (+ (Utilities|Struct|BreakItems _returnvalue_2) (LocalVariables|GetcurChanceGroup))) ; If we are lower or equal the ran num, get row.  \nOtherwise append drop chance and check again
          (bind _output_get (Variables|Components|SetlostItemData _returnvalue_2))
          (Components|StaticMesh|SetStaticMesh (Variables|Default|GetlostObject) (Utilities|Struct|BreakItems _output_get))
          (Physics|SetSimulatePhysics (Variables|Default|GetlostObject) true)
          (return)))))
  (Class|AutomationBlueprintFunctionLibrary|AddExpectedLogError "Did not find lost item")
  (return))

(fn HidefromView
  (Physics|SetSimulatePhysics (Variables|Default|GetlostObject) false)
  (Rendering|SetVisibility (Variables|Default|GetlostObject) false false)
  (Collision|SetCollisionEnabled (Variables|Default|GetlostObject) "NoCollision"))

(fn SnaptoSocket
  (params (socketHolder :type Actor%20Object%20Reference) (socketName :type Name)))

(fn DropatLocation
  (params (position :type Vector))
  (bind _returnvalue (Game|SpawnActorfromClass "lostItemV2_C" (Math|Transform|MakeTransform position "0, 0, 0" "1,1,1") "Undefined" 0 false 0))
  (Variables|lostItemV2_C|SetlostObject _returnvalue (Variables|Default|GetlostObject))
  (Components|StaticMesh|SetStaticMesh (Variables|lostItemV2_C|GetlostObject _returnvalue) (Variables|/Script/Engine.StaticMeshComponent|GetStaticMesh (Variables|Default|GetlostObject)))
  (Variables|lostItemV2_C|SetitemOwner _returnvalue (Variables|Components|GetitemOwner))
  (Variables|lostItemV2_C|SetlostItemData _returnvalue (Variables|Components|GetlostItemData))
  (Variables|lostItemV2_C|SetownerFound _returnvalue (Variables|Default|GetownerFound))
  (Actor|DestroyActor))