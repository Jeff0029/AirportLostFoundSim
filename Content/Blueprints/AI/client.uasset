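; Client AI character with a configurable shirt color, walk speed and type.
; When its capsule overlaps the first-person player, it nudges itself away, then switches on Type with no actions attached.
; The construction script creates a dynamic shirt material, which SetColor tints and applies to the torso.
; Helper functions set the movement speed and show the Type name on a debug text component.
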(event OnComponentBeginOverlap(CapsuleComponent)
  (params (OverlappedComponent :type Primitive%20Component%20Object%20Reference) (OtherActor :type Actor%20Object%20Reference) (OtherComp :type Primitive%20Component%20Object%20Reference) (OtherBodyIndex :type Integer) (bFromSweep :type Boolean) (SweepResult :type Hit%20Result%20Structure%20%28by%20ref%29))
  (bind _asfirst_person_character (Utilities|Casting|CastToFirstPersonCharacter OtherActor))
  (Transformation|AddActorWorldOffset self (* (Math|Vector|Normalize (- (Transformation|GetActorLocation) (Transformation|GetActorLocation _asfirst_person_character))) 5.0))
  (switch Utilities|FlowControl|Switch|SwitchonClientTypes (Variables|Default|Gettype)))

(event EventBeginPlay)

(event EventTick
  (params (DeltaSeconds :type Float%20%28single-precision%29)))

(fn ConstructionScript
  (bind _returnvalue (Rendering|Material|CreateDynamicMaterialInstance "/Game/Materials/Shirt.Shirt" "None" "None" :!class /Script/Engine.KismetMaterialLibrary))
  (Variables|Default|SetshirtMaterial _returnvalue))

(fn SetColor
  (params (newColor :type Linear%20Color%20Structure))
  (Rendering|Material|SetVectorParameterValue (Variables|Default|GetshirtMaterial) "Color" newColor :!class /Script/Engine.MaterialInstanceDynamic)
  (Rendering|Material|SetMaterial (Variables|Default|Gettorso) 0 (Variables|Default|GetshirtMaterial))
  (Variables|Default|SetshirtColor newColor))

(fn SetWalkSpeed
  (params (newSpeed :type Float%20%28single-precision%29))
  (Variables|/Script/Engine.CharacterMovementComponent|SetMaxWalkSpeed (Variables|Character|GetCharacterMovement) newSpeed))

(fn SetText
  (Rendering|Components|TextRender|SetText (Variables|Default|Get%28debug%29%20show%20Type) (Utilities|Text|ToText(String) (Utilities|String|EnumtoString (Variables|Default|Gettype)))))