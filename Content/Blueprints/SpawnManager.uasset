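; Spawn manager that populates the level with Client actors and drops LostItemV2 actors owned by them.
; On BeginPlay it spawns clients at random navigable spots, retrying failed spawns, cycling shirt colors and assigning types by cycling through the CLIENTTYPERATIO weights.
; HandleDrop, not started here, waits a random delay, then spawns an item at a random client and calls itself again while LostItems is within MAXLOSTITEM.
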(event Custom|HandleDrop
  (bind _possibledelay (Variables|Items|GetpossibleDelay))
  (bind _clients (Variables|Default|Getclients))
  (Utilities|FlowControl|Delay (Math|Random|RandomFloatinRange (.value (.lowerbound _possibledelay)) (.value (.upperbound _possibledelay))))
  (if (<= (Utilities|Array|Length (Variables|items|GetlostItems)) (Variables|Items|GetMAX_LOST_ITEM))
    (bind _output_get (Variables|Default|SetchosenOwner (Utilities|Array|Get(acopy) _clients (Math|Random|RandomIntegerinRange 0 (- (Utilities|Array|Length _clients) 1)))))
    (bind _returnvalue (Game|SpawnActorfromClass "/Game/Blueprints/lostItemV2.lostItemV2_C" (Math|Transform|MakeTransform (Transformation|GetActorLocation _output_get) "0, 0, 0" "1,1,1") "AdjustIfPossibleButAlwaysSpawn" 0 true 0))
    (Variables|/Game/Blueprints/lostItemV2.lostItemV2_C|SetitemOwner _returnvalue _output_get)
    (CallFunction|HandleDrop)))

(event EventBeginPlay
  (CallFunction|SpawnClients))

(event EventTick
  (params (DeltaSeconds :type Float%20%28single-precision%29)))

(fn SpawnClients
  (bind _returnvalue (Transformation|GetWorldLocation))
  (bind _randomlocation (Class|NavigationSystemV1|GetRandomPointinNavigableRadius _returnvalue 6.02e+03 0 0))
  (for _index (range 0 (- (Variables|Default|GetinitSpawnAmount) 1))
    (bind _returnvalue_2 (Game|SpawnActorfromClass "/Game/Blueprints/AI/client.client_C" (Math|Transform|MakeTransform (Math|Vector|MakeVector (.x _randomlocation) (.y _randomlocation) 5e+01) (Math|Rotator|MakeRotator 0.0 0.0 (Math|Random|RandomFloatinRange 0.0 359.0)) "1,1,1") "AdjustIfPossibleButDontSpawnIfColliding" 0 0 :!label _label))
    (Utilities|IsValid _returnvalue_2
      (:Is%20Valid
        (Default|SetColor _returnvalue_2 (Utilities|Array|Get(acopy) (Variables|Default|GetpossibleShirtColors) (Math|Integer|%(Integer) _index (Utilities|Array|Length (Variables|Default|GetpossibleShirtColors)))))
        (bind _clienttype (CallFunction|GetNextClientType))
        (Variables|/Game/Blueprints/AI/client.client_C|Settype _returnvalue_2 _clienttype)
        (Utilities|Array|Add (Variables|Default|Getclients) _returnvalue_2)
        (Default|SetText _returnvalue_2))
      (:Is%20Not%20Valid
        (goto _label)))))

(fn GetNextClientType
  (bind _values (Utilities|Map|Values (Variables|Default|GetCLIENT_TYPE_RATIO)))
  (for _array_element _values
    (LocalVariables|SettotalPerType (+ _array_element (LocalVariables|GettotalPerType))))
  (bind _keys (Utilities|Map|Keys (Variables|Default|GetCLIENT_TYPE_RATIO)))
  (for _array_element_2 _keys
    (LocalVariables|SetcurrentChecker (+ (LocalVariables|GetcurrentChecker) (.Value (Utilities|Map|Find (Variables|Default|GetCLIENT_TYPE_RATIO) _array_element_2))))
    (if (< (Math|Integer|%(Integer) (Utilities|Array|Length (Variables|Default|Getclients)) (LocalVariables|GettotalPerType)) (LocalVariables|GetcurrentChecker))
      (return _array_element_2))))